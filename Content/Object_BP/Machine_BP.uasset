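; Machine actor Blueprint with parts that spin through rotating movement components.
; Five RotatingMovement components each drive their own static mesh component, so the meshes can rotate independently.
; The pairings are reassigned with SetUpdatedComponent on every Tick rather than once at startup.
; The construction script is empty.
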(event EventTick
  (params (DeltaSeconds :type Float%20%28single-precision%29))
  (Components|Movement|SetUpdatedComponent (Variables|Default|GetRotatingMovement) (Variables|Default|GetStaticMeshComponent0))
  (Components|Movement|SetUpdatedComponent (Variables|Default|GetRotatingMovement1) (Variables|Default|GetStaticMeshComponent04))
  (Components|Movement|SetUpdatedComponent (Variables|Default|GetRotatingMovement2) (Variables|Default|GetStaticMeshComponent03))
  (Components|Movement|SetUpdatedComponent (Variables|Default|GetRotatingMovement3) (Variables|Default|GetStaticMeshComponent01))
  (Components|Movement|SetUpdatedComponent (Variables|Default|GetRotatingMovement4) (Variables|Default|GetStaticMeshComponent02)))

(fn ConstructionScript)